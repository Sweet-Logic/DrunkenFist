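; BP_shot is a 2D shot actor with a Paper2D flipbook that deals DamageShot damage to specific actors it overlaps, then destroys itself.
; On overlap, a sequence of casts picks the damage route by target class.
; BP_test and BP_test2 receive damage through their own DamageSystem function, while Enemy_Test receives it through the engine's ApplyDamage.
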(event `self.ReceiveBeginPlay`)

(event `self.ReceiveActorBeginOverlap`
  (params (OtherActor :type "Actor Object Reference"))
  (`|ExecutionSequence`
    (:`then_0`
      (bind _asbp_test (cast `/Game/Test/Blueprint/BP_test` OtherActor))
      (`/Game/Test/Blueprint/BP_test.damage system` _asbp_test (`self.damage shot`))
      (`self.K2_DestroyActor`))
    (:`then_1`
      (bind _asenemy_test (cast `/Game/Test/Blueprint/Enemy_Test` OtherActor))
      (`GameplayStatics.ApplyDamage` _asenemy_test (`self.damage shot`) (`self.GetInstigatorController` self) self "/Script/Engine.DamageType")
      (`self.K2_DestroyActor`))
    (:`then_2`
      (bind _asbp_test_2 (cast `/Game/Test/Blueprint/BP_test2` OtherActor))
      (`/Game/Test/Blueprint/BP_test2.damage system` _asbp_test_2 (`self.damage shot`))
      (`self.K2_DestroyActor`))))

(event `self.ReceiveTick`
  (params (DeltaSeconds :type "Float (single-precision)")))

(event `self.PaperFlipbook.OnComponentHit`
  (params (OtherActor :type "Actor Object Reference") (OtherComp :type "PrimitiveComponent Object Reference") (NormalImpulse :type "Vector Structure") (Hit :type "HitResult Structure (by ref)")))

(fn `UserConstructionScript`)