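; Player 1's Paper2D side-view fighter character with movement, jump, dash, shooting, blocking and a held power-up mode.
; A State enum selects the sprite flipbook, while horizontal velocity sets facing for dashes and knockback.
; Damage lowers health, disabling input on death or until a hit character lands and recovers.
; Tick regenerates stamina and power and drains block; power mode loops fire spawns and swaps normal shots for a rate-limited power shot.
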(event `damage system`
  (params (damagein :type "Float (double-precision)"))
  ;[1 1 1] damage
  (if (`self.bCanBeDamaged`) :!label _label
    (set `self.ishit` true)
    (`self.DisableInput` (`GameplayStatics.GetPlayerController` 0))
    (bind _output_get (set `self.Health_current` (- (`self.Health_current`) damagein)))
    (if (<= _output_get 0.0)
      (set `self.State` "NewEnumerator5")
      (`self.DisableInput` (`GameplayStatics.GetPlayerController` 0))
      (`self.UpdateAnimation`)
      (else
        (set `self.State` "NewEnumerator4")
        (`CharacterMovementComponent.AddForce` (`self.CharacterMovement`) (`KismetMathLibrary.MakeVector` (* (`self.facing`) (`self.Knockback`)) 0.0 5000000.0))))))

(event `back_attack`
  ;[1 1 1] damage
  (goto _label))

(event `InputAction|Jump-player 1`
  (params (Key :type "Key Structure" :default "AnyKey"))
  ;[1 1 1] Handle Jump
  (:`Pressed`
    (if (`self.power`)
      _
      (elif (not (`self.blocking`))
        (`self.Jump`)
        (set `self.State` "NewEnumerator2"))))
  (:`Released`
    (`self.StopJumping`)))

(event `self.ReceiveBeginPlay`
  ;[1 1 1] Handle Animation
  (`|ExecutionSequence`
    (:`then_0`
      (`ActorComponent.SetIsReplicated` (`self.Sprite`) true))
    (:`then_1`
      (bind _returnvalue (`|CreateWidget` "/Game/Test/Blueprint/HUD.HUD_C" (`GameplayStatics.GetPlayerController` 0)))
      (bind _output_get (set `self.healthbar` _returnvalue))
      (`UserWidget.AddToViewport` _output_get 0))))

(event `UpdateAnimation`
  ;[1 1 1] Handle Animation
  (switch `/Game/Test/Blueprint/Char_states` (`self.State`)
    (:`NewEnumerator0`
      (`PaperFlipbookComponent.SetFlipbook` (`self.Sprite`) (select `bool` (> (`KismetMathLibrary.VSize` (`self.GetVelocity`)) 0.0) :`false` "/Game/Test/Sprites/Character/ATest_Idle.ATest_Idle" :`true` "/Game/Test/Sprites/Character/ARun_Test.ARun_Test" :!type "PaperFlipbook Object Reference")))
    (:`NewEnumerator1`
      (`PaperFlipbookComponent.SetFlipbook` (`self.Sprite`) "/Game/Test/Sprites/Character/ARun_Test.ARun_Test"))
    (:`NewEnumerator2`
      (`PaperFlipbookComponent.SetFlipbook` (`self.Sprite`) "/Game/Test/Sprites/Character/Ajump_test.Ajump_test"))
    (:`NewEnumerator4`
      (`PaperFlipbookComponent.SetFlipbook` (`self.Sprite`) "/Game/Test/Sprites/Character/AHit_Test.AHit_Test"))
    (:`NewEnumerator5`
      (`PaperFlipbookComponent.SetFlipbook` (`self.Sprite`) "/Game/Test/Sprites/Character/ADead_Test.ADead_Test"))
    (:`NewEnumerator6`
      (`PaperFlipbookComponent.SetFlipbook` (`self.Sprite`) "/Game/Test/Sprites/Character/Asitting_Test.Asitting_Test"))
    (:`NewEnumerator7`
      (`PaperFlipbookComponent.SetFlipbook` (`self.Sprite`) "/Game/Test/Sprites/Character/Ashooting_test.Ashooting_test"))
    (:`NewEnumerator9`
      (`PaperFlipbookComponent.SetFlipbook` (`self.Sprite`) "/Game/Test/Sprites/Character/power/power_shot.power_shot"))
    (:`NewEnumerator10`
      (`PaperFlipbookComponent.SetFlipbook` (`self.Sprite`) "/Game/Test/Sprites/Character/block/block_flip.block_flip"))))

(event `InputAxis|MoveRight_player1`
  (params (AxisValue :type "Float (single-precision)"))
  ;[1 1 1] Handle movement
  (if (`self.power`)
    _
    (elif (not (`self.blocking`))
      (`self.AddMovementInput` (1.0 0.0 0.0) AxisValue))))

(event `self.OnLanded`
  (params (Hit :type "HitResult Structure (by ref)"))
  ;[1 1 1] landing
  (if (`self.blocking`)
    _
    (elif (`self.ishit`)
      (set `self.State` "NewEnumerator6")
      (`self.UpdateAnimation`)
      (`KismetSystemLibrary.Delay` 0.5)
      (set `self.ishit` false)
      (set `self.State` "NewEnumerator0")
      (`self.UpdateAnimation`)
      (`self.EnableInput` (`GameplayStatics.GetPlayerController` 0))
      (else
        (set `self.State` "NewEnumerator0")
        (`self.UpdateAnimation`)))))

(event `self.ReceiveTick`
  (params (DeltaSeconds :type "Float (single-precision)"))
  ;[1 1 1] Tick - Updates animation
  (`|ExecutionSequence`
    (:`then_0`
      (if (`self.shotting?`)
        (set `self.bCanBeDamaged` true)))
    (:`then_1`
      (`self.UpdateAnimation`)
      (`/Engine/EditorBlueprintResources/StandardMacros.CompareFloat` (.x (`MovementComponent.Velocity` (`self.GetMovementComponent`)))
        (:`>`
          (`Controller.SetControlRotation` (`self.GetController`) (`KismetMathLibrary.MakeRotator` 0.0 0.0 0.0))
          (set `self.facing` 1))
        (:`<`
          (`Controller.SetControlRotation` (`self.GetController`) (`KismetMathLibrary.MakeRotator` 0.0 0.0 180.0))
          (set `self.facing` -1))))
    (:`then_2`
      ;[0.8678 0.1104 1] block, power and stamina degrade/Regen
      (`KismetSystemLibrary.Delay` 5.0)
      (set `self.stamina` (`KismetMathLibrary.FClamp` (+ (`self.stamina`) 1.0))))
    (:`then_3`
      (if (`self.blocking`)
        (set `self.Block` (- (`self.Block`) 0.001))))
    (:`then_4`
      (if (<= (`self.Block`) 0.0)
        (set `self.bCanBeDamaged` true)
        (set `self.blocking` false)
        (set `self.State` "NewEnumerator0")))
    (:`then_5`
      (set `self.power_req` (`KismetMathLibrary.FClamp` (+ (`self.power_req`) 0.0005))))))

(event `Key|F`
  (params (Key :type "Key Structure" :default "AnyKey"))
  ;[1 0 0.9434] Dash
  (:`Pressed`
    (if (`self.power`)
      _
      (elif (`self.blocking`)
        _
        (elif (>= (`self.stamina`) 0.25)
          (`CharacterMovementComponent.AddForce` (`self.CharacterMovement`) (`KismetMathLibrary.MakeVector` (* (`self.facing`) (`self.Knockback`)) 0.0 0.0))
          (set `self.stamina` (- (`self.stamina`) 0.25)))))))

(event `Key|R`
  (params (Key :type "Key Structure" :default "AnyKey"))
  ;[0.009985 1 0] blocking
  (:`Pressed`
    (if (`self.power`)
      (set `self.bCanBeDamaged` true :!label _label_2)
      (set `self.blocking` false)
      (set `self.State` "NewEnumerator0")
      (`Widget.RemoveFromParent` (stale _returnvalue))
      (`KismetSystemLibrary.Delay` 10.0)
      (if (`self.blocking`)
        (set `self.Block` 1.0))
      (elif (>= (`self.Block`) 0.01)
        (set `self.bCanBeDamaged` false)
        (set `self.blocking` true)
        (set `self.State` "NewEnumerator10")
        (bind _returnvalue (`|CreateWidget` "/Game/Test/Blueprint/Block.Block_C"))
        (`UserWidget.AddToViewport` _returnvalue 0))))
  (:`Released`
    (goto _label_2)))

(event `Key|E`
  (params (Key :type "Key Structure" :default "AnyKey"))
  ;[1 0 0] Shootin
  (:`Pressed`
    (set `self.shotting?` true)
    (if (`self.power`)
      (`/Engine/EditorBlueprintResources/StandardMacros.DoOnce` false :!label _label_3
        (:`Completed`
          (`|SpawnActorFromClass` "/Game/Test/Blueprint/power.power_C" (`SceneComponent.K2_GetComponentToWorld` (`self.Arrow2`)) "Undefined" "OverrideRootScale")
          (set `self.State` "NewEnumerator9")
          (`self.UpdateAnimation`)
          (set `self.power_req` (- (`self.power_req`) 0.5))
          (`KismetSystemLibrary.RetriggerableDelay` 5.0)
          (`self.shot recharge`)))
      (else
        (`|SpawnActorFromClass` "/Game/Test/Blueprint/BP_shot.BP_shot_C" (`SceneComponent.K2_GetComponentToWorld` (`self.Arrow1`)) "Undefined" "OverrideRootScale")
        (set `self.State` "NewEnumerator7")
        (`self.UpdateAnimation`))))
  (:`Released`
    (`KismetSystemLibrary.RetriggerableDelay` 0.5)
    (set `self.State` "NewEnumerator0")
    (set `self.shotting?` false)))

(event `shot recharge`
  ;[1 0 0] Shootin
  (goto _label_3 :!via `Reset`))

(event `Key|Q`
  (params (Key :type "Key Structure" :default "AnyKey"))
  ;[0 1 0.9582] powerup
  (:`Pressed`
    (if (`self.blocking`)
      _
      (elif (>= (`self.power_req`) 0.1)
        (`PaperFlipbookComponent.SetSpriteColor` (`self.Sprite`) (`KismetMathLibrary.MakeColor` 0.0 0.6 1.0))
        (bind _returnvalue (`|CreateWidget` "/Game/Test/Blueprint/power_bar.power_bar_C"))
        (`UserWidget.AddToViewport` _returnvalue 0)
        (set `self.power` true)
        (`|ExecutionSequence` :!label _label_4
          (:`then_0`
            (`KismetSystemLibrary.Delay` 0.2)
            (`|SpawnActorFromClass` "/Game/Test/Blueprint/fire.fire_C" (`SceneComponent.K2_GetComponentToWorld` (`self.fire 1`)) "Undefined" "OverrideRootScale"))
          (:`then_1`
            (`KismetSystemLibrary.Delay` 1.0)
            (`|SpawnActorFromClass` "/Game/Test/Blueprint/fire.fire_C" (`SceneComponent.K2_GetComponentToWorld` (`self.fire 2`)) "Undefined" "OverrideRootScale"))
          (:`then_2`
            (`KismetSystemLibrary.Delay` 1.4)
            (`|SpawnActorFromClass` "/Game/Test/Blueprint/fire.fire_C" (`SceneComponent.K2_GetComponentToWorld` (`self.fire 3`)) "Undefined" "OverrideRootScale")
            (`self.fire loop`))))))
  (:`Released`
    (`PaperFlipbookComponent.SetSpriteColor` (`self.Sprite`) (`KismetMathLibrary.MakeColor` 1.0 1.0 1.0))
    (set `self.power` false)
    (`Widget.RemoveFromParent` _returnvalue)))

(event `fire loop`
  ;[0 1 0.9582] powerup
  (if (`self.power`)
    (goto _label_4)))

(fn `UserConstructionScript`)