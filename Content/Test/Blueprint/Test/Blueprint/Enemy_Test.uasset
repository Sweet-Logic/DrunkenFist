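; Test enemy Blueprint that deals damage on contact and dies when its health runs out.
; Beginning an actor overlap with BP_test passes its damage variable to that actor's DamageSystem.
; When a power or BP_shot ends overlap with its component, it subtracts that actor's DamageShot from health and destroys itself at zero or below.
; Its own damagesystem event is empty, so damage is handled directly in the overlap logic.
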(event `damage system`
  (params (damagein :type "Float (double-precision)")))

(event `self.ReceiveBeginPlay`)

(event `self.ReceiveActorBeginOverlap`
  (params (OtherActor :type "Actor Object Reference"))
  (`|ExecutionSequence`
    (:`then_0`
      (bind _asbp_test (cast `/Game/Test/Blueprint/BP_test` OtherActor))
      (`/Game/Test/Blueprint/BP_test.damage system` _asbp_test (`self.damagevariable`)))))

(event `self.ReceiveTick`
  (params (DeltaSeconds :type "Float (single-precision)")))

(event `self.  .OnComponentEndOverlap`
  (params (OtherActor :type "Actor Object Reference") (OtherComp :type "PrimitiveComponent Object Reference") (OtherBodyIndex :type Integer))
  (`|ExecutionSequence`
    (:`then_0`
      (bind _aspower (cast `/Game/Test/Blueprint/power` OtherActor))
      (bind _output_get (set `self.Health current` (- (`self.Health current`) (`/Game/Test/Blueprint/power.damage shot` _aspower))))
      (if (<= _output_get 0.0)
        (`self.K2_DestroyActor`)))
    (:`then_1`
      (bind _asbp_shot (cast `/Game/Test/Blueprint/BP_shot` OtherActor))
      (bind _output_get_2 (set `self.Health current` (- (`self.Health current`) (`/Game/Test/Blueprint/BP_shot.damage shot` _asbp_shot))))
      (if (<= _output_get_2 0.0)
        (`self.K2_DestroyActor`)))))

(fn `UserConstructionScript`)