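; Test player controller for player one that sets up a second controllable character for local two-player movement.
; On BeginPlay it spawns a Player2 controller and a BP_test2 character owned by it, then has that controller possess the character.
; It handles both players' horizontal input axes itself, moving its own pawn and the stored second character along world X.
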(event `self.ReceiveBeginPlay`
  (bind _returnvalue (`KismetMathLibrary.MakeTransform` (53.0 0.0 52.0)))
  (`KismetSystemLibrary.PrintString` "Hello" true true (struct :`R` 1.0 :`G` 0.063895 :`A` 1.0))
  (bind _returnvalue_2 (`|SpawnActorFromClass` "/Game/Test/Blueprint/player2.player2_C" _returnvalue "Undefined" "OverrideRootScale"))
  (bind _output_get (set `self.second controller` _returnvalue_2))
  (bind _returnvalue_3 (`|SpawnActorFromClass` "/Game/Test/Blueprint/BP_test2.BP_test2_C" _returnvalue "Undefined" "OverrideRootScale" _output_get))
  (set `self.second char` _returnvalue_3)
  (`self.Possess` (`self.second controller`) (`self.second char`)))

(event `InputAxis|MoveRight_player1`
  (params (AxisValue :type "Float (single-precision)"))
  (`Pawn.AddMovementInput` (`self.K2_GetPawn`) (1.0 0.0 0.0) AxisValue false))

(event `InputAxis|Moveright_player2`
  (params (AxisValue :type "Float (single-precision)"))
  (`Pawn.AddMovementInput` (`self.second char`) (1.0 0.0 0.0) AxisValue false))

(fn `UserConstructionScript`)