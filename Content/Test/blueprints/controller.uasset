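; Player controller for a local two-player 2D side-scroller, handling movement for both characters from one controller.
; On BeginPlay it spawns a second controller and character, possesses that character, and caches the first player's character.
; Axis inputs move, animate and turn each character; player 2's jump, shoot and dash inputs are forwarded directly to its pawn.
; Tick creates and adds a new HUD widget every frame.
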(event `self.ReceiveBeginPlay`
  (bind _returnvalue (`KismetMathLibrary.MakeTransform` (-662.0 -13.0 390.0)))
  (`|ExecutionSequence`
    (:`then_0`
      (bind _returnvalue_2 (`|SpawnActorFromClass` "/Game/Test/blueprints/controller2.controller2_C" _returnvalue))
      (set `self.controller2` _returnvalue_2)
      (bind _returnvalue_3 (`|SpawnActorFromClass` "/Game/Test/blueprints/2DSideScrollerCharacter2.2DSideScrollerCharacter2_C" _returnvalue))
      (set `self.player 2` _returnvalue_3)
      (`self.Possess` (`self.controller2`) (`self.player 2`)))
    (:`then_1`
      (bind _as2dside_scroller_character (cast `/Game/Test/blueprints/2DSideScrollerCharacter` (`GameplayStatics.GetPlayerCharacter` 0)))
      (set `self.2sacroll` _as2dside_scroller_character))
    (:`then_2`
      (bind _as2dside_scroller_character_2 (cast `/Game/Test/blueprints/2DSideScrollerCharacter2` (`GameplayStatics.GetPlayerCharacter` 0)))
      (set `self.3sacroll` _as2dside_scroller_character_2))))

(event `InputAxis|MoveRight`
  (params (AxisValue :type "Float (single-precision)"))
  (bind _2sacroll (`self.2sacroll`))
  (`Pawn.AddMovementInput` (`self.K2_GetPawn`) (1.0 0.0 0.0) AxisValue false)
  (`/Game/Test/blueprints/2DSideScrollerCharacter.UpdateAnimation` (`self.2sacroll`))
  (`/Engine/EditorBlueprintResources/StandardMacros.CompareFloat` AxisValue
    (:`>`
      (`self.SetControlRotation` (`KismetMathLibrary.MakeRot` 0.0 0.0))
      (`/Game/Test/blueprints/2DSideScrollerCharacter.facing 1` _2sacroll))
    (:`<`
      (`self.SetControlRotation` (`KismetMathLibrary.MakeRot` 0.0 180.0))
      (`/Game/Test/blueprints/2DSideScrollerCharacter.facing -1` _2sacroll))))

(event `InputAxis|move right 2`
  (params (AxisValue :type "Float (single-precision)"))
  (bind _player_2 (`self.player 2`))
  (bind _player_2_2 (`self.player 2`))
  (bind _player_2_3 (`self.player 2`))
  (`Pawn.AddMovementInput` _player_2 (1.0 0.0 0.0) AxisValue false)
  (`/Game/Test/blueprints/2DSideScrollerCharacter2.UpdateAnimation` _player_2)
  (`/Engine/EditorBlueprintResources/StandardMacros.CompareFloat` AxisValue
    (:`>`
      (`self.SetActorRotation` _player_2_2 (`KismetMathLibrary.MakeRot` 0.0 0.0))
      (`/Game/Test/blueprints/2DSideScrollerCharacter2.player 2 facing 1` _player_2_3))
    (:`<`
      (`self.SetActorRotation` _player_2_2 (`KismetMathLibrary.MakeRot` 0.0 180.0))
      (`/Game/Test/blueprints/2DSideScrollerCharacter2.player 2 facign -1` _player_2_3))))

(event `InputAction|Jump2`
  (bind _player_2 (`self.player 2`))
  ;[1 1 1] player 2 button presses
  (:`Pressed`
    (`Character.Jump` _player_2)
    (`/Game/Test/blueprints/2DSideScrollerCharacter2.jump start` _player_2))
  (:`Released`
    (`Character.StopJumping` _player_2)
    (`/Game/Test/blueprints/2DSideScrollerCharacter2.jump end` _player_2)))

(event `Key|Y`
  (bind _player_2 (`self.player 2`))
  ;[1 1 1] player 2 button presses
  (:`Pressed`
    (`/Game/Test/blueprints/2DSideScrollerCharacter2.player 2 shoot` _player_2))
  (:`Released`
    (`/Game/Test/blueprints/2DSideScrollerCharacter2.player 2 end shoot` _player_2)))

(event `Key|U`
  ;[1 1 1] player 2 button presses
  (:`Pressed`
    (`/Game/Test/blueprints/2DSideScrollerCharacter2.player 2 dash` (`self.player 2`))))

(event `self.ReceiveTick`
  (params (DeltaSeconds :type "Float (single-precision)"))
  (bind _returnvalue (`|CreateWidget` "/Game/Test/blueprints/Widget/HUD.HUD_C"))
  (`UserWidget.AddToViewport` _returnvalue 0))

(fn `UserConstructionScript`)